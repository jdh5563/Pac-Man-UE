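; Game mode for two-player Pac-Man that runs level setup, ghost resets and a shared point total.
; BeginPlay generates the level, possesses a Pac-Man per player at PlayerStarts, then duplicates walls, collectibles and teleports at an X offset.
; SpawnGhosts repositions existing ghosts and assigns their target player index by actor tag.
; Tick regenerates the level when the tracked pellet array empties, resetting only player 0's Pac-Man alongside the ghosts.
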(event Custom|Regenerate%20Level
  ;[1 1 1] Regenerate the level
  (bind _outactors (Actor|GetAllActorsOfClass "/Game/Blueprints/BP_Wall.BP_Wall_C"))
  (for _array_element _outactors
    (Actor|DestroyActor _array_element))
  (Class|LevelGenerator|GenerateLevel (Variables|Default|GetLevelGenerator) "/Game/Blueprints/BP_Wall.BP_Wall_C" "/Game/Blueprints/Collectibles/BP_Pellet.BP_Pellet_C" "/Game/Blueprints/Collectibles/BP_PowerPellet.BP_PowerPellet_C" "/Game/Blueprints/BP_Teleport.BP_Teleport_C")
  (bind _outactors_2 (Actor|GetAllActorsOfClass "/Game/Blueprints/Collectibles/BP_Collectible.BP_Collectible_C"))
  (Variables|Default|SetPellets _outactors_2)
  (bind _asbp_pac_man (Utilities|Casting|CastToBP_PacMan (Game|Player|GetPlayerPawn 0)))
  (CallFunction|SpawnGhosts)
  (Default|ResettoSpawn _asbp_pac_man))

(event Custom|SpawnGhosts
  ;[1 1 1] Set ghost locations
  (for _array_element (Variables|Default|GetGhosts)
    (bind _asbp_ghost (Utilities|Casting|CastToBP_Ghost _array_element))
    (bind _asbp_ghost_controller (Utilities|Casting|CastToBP_GhostController (Pawn|GetController _asbp_ghost)))
    (Variables|/Game/Blueprints/Ghost/Controllers/BP_GhostController.BP_GhostController_C|SetIsScattering _asbp_ghost_controller false)
    (Transformation|SetActorLocation _array_element (Variables|/Game/Blueprints/Ghost/Pawns/BP_Ghost.BP_Ghost_C|GetStartLocation _asbp_ghost) false false)
    (if (== (Utilities|Array|Get(acopy) (Variables|/Script/Engine.Actor|GetTags _asbp_ghost)) "P0")
      (Variables|/Game/Blueprints/Ghost/Controllers/BP_GhostController.BP_GhostController_C|SetPlayerIndex _asbp_ghost_controller 0)
      (else
        (Variables|/Game/Blueprints/Ghost/Controllers/BP_GhostController.BP_GhostController_C|SetPlayerIndex _asbp_ghost_controller 1)))))

(event Custom|SetDelays
  ;[1 1 1] Set everything to delay.
  (for _array_element (Variables|Default|GetGhosts)
    (Variables|/Game/Blueprints/Ghost/Controllers/BP_GhostController.BP_GhostController_C|SetShouldDelay (Variables|/Game/Blueprints/Ghost/Pawns/BP_Ghost.BP_Ghost_C|GetGhostController _array_element) true)
    (bind _asbp_pac_man (Utilities|Casting|CastToBP_PacMan (Game|Player|GetPlayerPawn 0)))
    (Variables|/Game/Blueprints/CharacterPawns/BP_PacMan.BP_PacMan_C|SetshouldDelay _asbp_pac_man true)))

(event EventBeginPlay
  (bind _levelcopy (Variables|Default|GetLevelCopy))
  ;[1 1 1] Setting level generator reference and generating the level.
  (bind _returnvalue (Actor|GetActorOfClass "/Script/PacMan.LevelGenerator"))
  (bind _output_get (Variables|Default|SetLevelGenerator _returnvalue))
  (Class|LevelGenerator|GenerateLevel _output_get "/Game/Blueprints/BP_Wall.BP_Wall_C" "/Game/Blueprints/Collectibles/BP_Pellet.BP_Pellet_C" "/Game/Blueprints/Collectibles/BP_PowerPellet.BP_PowerPellet_C" "/Game/Blueprints/BP_Teleport.BP_Teleport_C")
  ;[1 1 1] Tracking all the pellets in the level.
  (bind _outactors (Actor|GetAllActorsOfClass "/Game/Blueprints/Collectibles/BP_Collectible.BP_Collectible_C"))
  (Variables|Default|SetPellets _outactors)
  ;[1 1 1] Getting a reference to all ghosts and setting their location.
  (bind _outactors_2 (Actor|GetAllActorsOfClass "/Game/Blueprints/Ghost/Pawns/BP_Ghost.BP_Ghost_C"))
  (for _array_element _outactors_2
    (Utilities|Array|Add (Variables|Default|GetGhosts) _array_element))
  ;[1 1 1] Spawning in a second pac man pawn
  (bind _outactors_3 (Actor|GetAllActorsOfClass "/Script/Engine.PlayerStart"))
  (for _index (range 0 1)
    (Class|GameplayStatics|CreatePlayer _index)
    (bind _returnvalue_2 (Game|SpawnActorfromClass "/Game/Blueprints/CharacterPawns/BP_PacMan.BP_PacMan_C" (Transformation|GetActorTransform (Utilities|Array|Get(acopy) _outactors_3 _index)) "AlwaysSpawn" "MultiplyWithRoot" 0 0))
    (Variables|/Game/Blueprints/CharacterPawns/BP_PacMan.BP_PacMan_C|SetplayerIndex _returnvalue_2 _index)
    (Pawn|Possess (Game|GetPlayerController _index) _returnvalue_2)
    (CallFunction|SpawnGhosts))
  (Audio|PlaySound2D "/Game/Sounds/pacman_beginning.pacman_beginning" 1.0 1.0 0.0 0 0)
  ;[1 1 1] Creating a copy of the level and moving it over.
  (bind _outactors_4 (Actor|GetAllActorsOfClass "/Game/Blueprints/Collectibles/BP_Collectible.BP_Collectible_C"))
  (for _array_element_2 _outactors_4
    (Utilities|Array|Add _levelcopy _array_element_2))
  (bind _outactors_5 (Actor|GetAllActorsOfClass "/Game/Blueprints/BP_Wall.BP_Wall_C"))
  (for _array_element_3 _outactors_5
    (Utilities|Array|Add _levelcopy _array_element_3))
  (bind _outactors_6 (Actor|GetAllActorsOfClass "/Game/Blueprints/BP_Teleport.BP_Teleport_C"))
  (for _array_element_4 _outactors_6
    (Utilities|Array|Add _levelcopy _array_element_4))
  (for _array_element_5 _levelcopy
    (Game|SpawnActorfromClass (Utilities|GetClass _array_element_5) (Math|Transform|MakeTransform (+ (.location (Transformation|GetActorTransform _array_element_5)) "6000.000000,0.000000,0.000000") (.rotation (Transformation|GetActorTransform _array_element_5)) (.scale (Transformation|GetActorTransform _array_element_5))) "AlwaysSpawn" "MultiplyWithRoot" 0 0)))

(event EventTick
  (params (DeltaSeconds :type Float%20%28single-precision%29))
  ;[1 1 1] Handling when there are no more pellets to collect.
  (if (== (Utilities|Array|Length (Variables|Default|GetPellets)) 0)
    (CallFunction|RegenerateLevel)))

(fn ConstructionScript)

(fn AddPoints
  (params (pointsToAdd :type Integer))
  (Variables|Default|SettotalPoints (+ pointsToAdd (Variables|Default|GettotalPoints))))