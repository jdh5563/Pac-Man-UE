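; BP_Ghost is a ghost pawn whose sphere changes appearance while the ghost is scattering.
; On BeginPlay it caches the Sphere's first material as the base, provided that casts to Material.
; Every Tick it reads IsScattering from its BP_GhostController and sets the Sphere to either M_Scatter or the cached base material.
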(event EventTick
  (params (DeltaSeconds :type Float%20%28single-precision%29))
  (bind _sphere (Variables|Default|GetSphere))
  ;[1 1 1] Change the material between base and scatter
  (bind _asbp_ghost_controller (Utilities|Casting|CastToBP_GhostController (Pawn|GetController)))
  (if (Variables|/Game/Blueprints/Ghost/Controllers/BP_GhostController.BP_GhostController_C|GetIsScattering _asbp_ghost_controller)
    (Rendering|Material|SetMaterial _sphere 0 "/Game/Materials/M_Scatter.M_Scatter")
    (else
      (Rendering|Material|SetMaterial _sphere 0 (Variables|Default|GetBaseMaterial)))))

(event EventBeginPlay
  ;[1 1 1] Set the base material
  (bind _asmaterial (Utilities|Casting|CastToMaterial (Rendering|Material|GetMaterial (Variables|Default|GetSphere) 0)))
  (Variables|Default|SetBaseMaterial _asmaterial))

(fn ConstructionScript)