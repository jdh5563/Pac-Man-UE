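; Ghost controller for Inky that sets a chase target from the positions of PacMan and Blinky.
; On BeginPlay it finds Blinky and starts a looping timer that runs Chase at the configured update delay.
; Chase projects a look-ahead point along PacMan's horizontal or vertical move direction.
; The target lands two units from Blinky toward that point, as the Blinky-to-point vector is normalized before doubling.
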(event Custom|Chase
  (bind _blinky (Variables|Default|GetBlinky))
  (bind _blinky_2 (Variables|Default|GetBlinky))
  (bind _returnvalue (Transformation|GetActorLocation _blinky_2))
  (bind _returnvalue_2 (Transformation|GetActorLocation _blinky))
  ;[1 1 1] Check the direction PacMan is moving
  (bind _asbp_pac_man (Utilities|Casting|CastToBP_PacMan (Game|Player|GetPlayerPawn 0)))
  (if (!= (.x (Variables|/Game/Blueprints/CharacterPawns/BP_PacMan.BP_PacMan_C|GetmoveDirection _asbp_pac_man)) 0.0)
    (Variables|Default|SetTargetLocation (+ (* (Math|Vector|Normalize (- (+ (Transformation|GetWorldLocation (Variables|/Game/Blueprints/CharacterPawns/BP_PacMan.BP_PacMan_C|GetSphere _asbp_pac_man)) (Math|Vector|MakeVector (* (.x (Variables|/Game/Blueprints/CharacterPawns/BP_PacMan.BP_PacMan_C|GetmoveDirection _asbp_pac_man)) (Variables|Default|GetLookAheadDistance)) 0.0 0.0)) _returnvalue)) 2.0) _returnvalue))
    (else
      (Variables|Default|SetTargetLocation (+ (* (Math|Vector|Normalize (- (+ (Transformation|GetWorldLocation (Variables|/Game/Blueprints/CharacterPawns/BP_PacMan.BP_PacMan_C|GetSphere _asbp_pac_man)) (Math|Vector|MakeVector 0.0 (* (.y (Variables|/Game/Blueprints/CharacterPawns/BP_PacMan.BP_PacMan_C|GetmoveDirection _asbp_pac_man)) (Variables|Default|GetLookAheadDistance)) 0.0)) _returnvalue_2)) 2.0) _returnvalue_2)))))

(event EventBeginPlay
  ;[1 1 1] Get a reference to Blinky then update target location on a delay
  (|CallParentFunction)
  (bind _returnvalue (Actor|GetActorOfClass "/Game/Blueprints/Ghost/Pawns/BP_Blinky.BP_Blinky_C"))
  (Variables|Default|SetBlinky _returnvalue)
  (Utilities|Time|SetTimerbyEvent (delegate Custom|Chase) (Variables|Default|GetChaseUpdateDelay) true))

(fn ConstructionScript
  (|CallParentFunction))