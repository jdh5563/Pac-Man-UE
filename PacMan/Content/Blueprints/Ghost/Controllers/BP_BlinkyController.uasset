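; Controller for Blinky, the ghost that directly chases Pac-Man.
; On BeginPlay it starts a looping timer that fires Chase every ChaseUpdateDelay seconds, so Tick stays empty.
; Each Chase sends the controlled pawn via AIMoveTo to the current world location of the Sphere component on the player's BP_PacMan, stopping on overlap.
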(event Custom|Chase
  (bind _asbp_pac_man (Utilities|Casting|CastToBP_PacMan (Game|Player|GetPlayerPawn 0)))
  (AI|AIMoveTo (Pawn|GetControlledPawn) (Transformation|GetWorldLocation (Variables|/Game/Blueprints/BP_PacMan.BP_PacMan_C|GetSphere _asbp_pac_man)) 0 5.0 true))

(event EventBeginPlay
  (Utilities|Time|SetTimerbyEvent (delegate Custom|Chase) (Variables|Default|GetChaseUpdateDelay) true))

(event EventTick
  (params (DeltaSeconds :type Float%20%28single-precision%29)))

(fn ConstructionScript
  (|CallParentFunction))