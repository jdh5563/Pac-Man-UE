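; Controller for the Pinky ghost that aims ahead of Pac-Man to ambush the player.
; On BeginPlay it starts a looping timer that refreshes the chase target every ChaseUpdateDelay seconds.
; Each update offsets the target from Pac-Man's sphere location by LookAheadDistance along the current move direction, using X when horizontal movement is present and Y otherwise.
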(event Custom|Chase
  ;[1 1 1] Check the direction PacMan is moving
  (bind _asbp_pac_man (Utilities|Casting|CastToBP_PacMan (Game|Player|GetPlayerPawn (Variables|Default|GetPlayerIndex))))
  (if (!= (.x (Variables|/Game/Blueprints/CharacterPawns/BP_PacMan.BP_PacMan_C|GetmoveDirection _asbp_pac_man)) 0.0)
    ;[1 1 1] Move left or right
    (Variables|Default|SetTargetLocation (+ (Transformation|GetWorldLocation (Variables|/Game/Blueprints/CharacterPawns/BP_PacMan.BP_PacMan_C|GetSphere _asbp_pac_man)) (Math|Vector|MakeVector (* (.x (Variables|/Game/Blueprints/CharacterPawns/BP_PacMan.BP_PacMan_C|GetmoveDirection _asbp_pac_man)) (Variables|Default|GetLookAheadDistance)) 0.0 0.0)))
    (else
      ;[1 1 1] Move up or down
      (Variables|Default|SetTargetLocation (+ (Transformation|GetWorldLocation (Variables|/Game/Blueprints/CharacterPawns/BP_PacMan.BP_PacMan_C|GetSphere _asbp_pac_man)) (Math|Vector|MakeVector 0.0 (* (.y (Variables|/Game/Blueprints/CharacterPawns/BP_PacMan.BP_PacMan_C|GetmoveDirection _asbp_pac_man)) (Variables|Default|GetLookAheadDistance)) 0.0))))))

(event EventBeginPlay
  ;[1 1 1] Update target location on a delay
  (|CallParentFunction)
  (Utilities|Time|SetTimerbyEvent (delegate Custom|Chase) (Variables|Default|GetChaseUpdateDelay) true))

(fn ConstructionScript
  (|CallParentFunction))