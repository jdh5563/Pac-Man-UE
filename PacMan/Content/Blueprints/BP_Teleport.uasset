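; Side tunnel teleporter for a Pac-Man game that moves Pac-Man and ghosts to its paired teleporter.
; After a one-second delay, it reads its "Left" tag and searches the Levels array of whichever player's Pac-Man owns it for another teleporter at the same Y.
; On box overlap, it places the actor at that partner, offset according to the partner's side, presumably to avoid retriggering.
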(event OnComponentBeginOverlap(Box)
  (params (OverlappedComponent :type Primitive%20Component%20Object%20Reference) (OtherActor :type Actor%20Object%20Reference) (OtherComp :type Primitive%20Component%20Object%20Reference) (OtherBodyIndex :type Integer) (bFromSweep :type Boolean) (SweepResult :type Hit%20Result%20Structure%20%28by%20ref%29))
  (bind _oppositeteleport (Variables|Default|GetOppositeTeleport))
  (bind _oppositeteleport_2 (Variables|Default|GetOppositeTeleport))
  (bind _spawnoffsetvector (Variables|Default|GetSpawnOffsetVector))
  (bind _spawnoffsetvector_2 (Variables|Default|GetSpawnOffsetVector))
  (bind _returnvalue (Transformation|GetActorLocation _oppositeteleport_2))
  (bind _returnvalue_2 (Transformation|GetActorLocation _oppositeteleport))
  (Utilities|FlowControl|Sequence
    (:then_0
      ;[1 0.8046 0.1394] Checking for collisions with PacMan and teleporting them.
      (if (== (Utilities|GetClass OtherActor) "/Game/Blueprints/CharacterPawns/BP_PacMan.BP_PacMan_C")
        (bind _asbp_pac_man (Utilities|Casting|CastToBP_PacMan OtherActor))
        (if (Variables|BP_Teleport_C|GetIsLeft _oppositeteleport_2)
          (Transformation|SetActorLocation _asbp_pac_man (+ _returnvalue _spawnoffsetvector_2) false true)
          (else
            (Transformation|SetActorLocation _asbp_pac_man (- _returnvalue _spawnoffsetvector_2) false true)))))
    (:then_1
      ;[1 0 0.009844] Checking for collisions with ghosts and teleporting them
      (if (Utilities|ClassIsChildOf (Utilities|GetClass OtherActor) "/Game/Blueprints/Ghost/Pawns/BP_Ghost.BP_Ghost_C")
        (bind _asbp_ghost (Utilities|Casting|CastToBP_Ghost OtherActor))
        (if (Variables|BP_Teleport_C|GetIsLeft _oppositeteleport)
          (Transformation|SetActorLocation _asbp_ghost (+ _returnvalue_2 _spawnoffsetvector) false false)
          (else
            (Transformation|SetActorLocation _asbp_ghost (- _returnvalue_2 _spawnoffsetvector) false false)))))))

(event EventBeginPlay
  (Utilities|FlowControl|Delay 1.0)
  (if (== (Utilities|Array|Get(acopy) (Variables|Actor|GetTags)) "Left")
    (Variables|Default|SetIsLeft true))
  ;[1 1 1] Setting the opposite side teleporter.
  (bind _asbp_pac_man (Utilities|Casting|CastToBP_PacMan (Game|Player|GetPlayerPawn 0)))
  (if (Utilities|Array|ContainsItem (Variables|/Game/Blueprints/CharacterPawns/BP_PacMan.BP_PacMan_C|Getlevels _asbp_pac_man) self)
    (Utilities|SetOppositeTeleporter (Variables|/Game/Blueprints/CharacterPawns/BP_PacMan.BP_PacMan_C|Getlevels _asbp_pac_man))
    (else
      (bind _asbp_pac_man_2 (Utilities|Casting|CastToBP_PacMan (Game|Player|GetPlayerPawn 1)))
      (Utilities|SetOppositeTeleporter (Variables|/Game/Blueprints/CharacterPawns/BP_PacMan.BP_PacMan_C|Getlevels _asbp_pac_man_2)))))

(fn ConstructionScript)