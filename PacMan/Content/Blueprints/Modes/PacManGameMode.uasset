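; Pac-Man game mode that builds the maze, restarts it once all pellets are gone and keeps the score.
; On BeginPlay it has the LevelGenerator spawn walls, pellets, teleports and ghosts, then caches all collectibles.
; Tick polls that array; when empty, it destroys the walls, regenerates the level, recaches collectibles and moves Pac-Man's sphere to the spawn location.
; AddPoints accumulates the total, while OnDeath is an empty stub.
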(event Custom|Regenerate%20Level
  ;[1 1 1] Regenerate the level
  (bind _outactors (Actor|GetAllActorsOfClass "/Game/Blueprints/BP_Wall.BP_Wall_C"))
  (for _array_element _outactors
    (Actor|DestroyActor _array_element))
  (Class|LevelGenerator|GenerateLevel (Variables|Default|GetLevelGenerator) "/Game/Blueprints/BP_Wall.BP_Wall_C" "/Game/Blueprints/Collectibles/BP_Pellet.BP_Pellet_C" "/Game/Blueprints/Collectibles/BP_PowerPellet.BP_PowerPellet_C" "/Game/Blueprints/BP_Teleport.BP_Teleport_C" "/Game/Blueprints/Ghost/Pawns/BP_Blinky.BP_Blinky_C" "/Game/Blueprints/Ghost/Pawns/BP_Inky.BP_Inky_C" "/Game/Blueprints/Ghost/Pawns/BP_Pinky.BP_Pinky_C" "/Game/Blueprints/Ghost/Pawns/BP_Clyde.BP_Clyde_C")
  (bind _outactors_2 (Actor|GetAllActorsOfClass "/Game/Blueprints/Collectibles/BP_Collectible.BP_Collectible_C"))
  (Variables|Default|SetPellets _outactors_2)
  (bind _asbp_pac_man (Utilities|Casting|CastToBP_PacMan (Game|Player|GetPlayerPawn 0)))
  (Transformation|SetWorldLocation (Variables|/Game/Blueprints/BP_PacMan.BP_PacMan_C|GetSphere _asbp_pac_man) (Variables|Default|GetSpawnLocation) false false))

(event EventBeginPlay
  ;[1 1 1] Setting level generator reference and generating the level.
  (bind _returnvalue (Actor|GetActorOfClass "/Script/PacMan.LevelGenerator"))
  (bind _output_get (Variables|Default|SetLevelGenerator _returnvalue))
  (Class|LevelGenerator|GenerateLevel _output_get "/Game/Blueprints/BP_Wall.BP_Wall_C" "/Game/Blueprints/Collectibles/BP_Pellet.BP_Pellet_C" "/Game/Blueprints/Collectibles/BP_PowerPellet.BP_PowerPellet_C" "/Game/Blueprints/BP_Teleport.BP_Teleport_C" "/Game/Blueprints/Ghost/Pawns/BP_Blinky.BP_Blinky_C" "/Game/Blueprints/Ghost/Pawns/BP_Inky.BP_Inky_C" "/Game/Blueprints/Ghost/Pawns/BP_Pinky.BP_Pinky_C" "/Game/Blueprints/Ghost/Pawns/BP_Clyde.BP_Clyde_C")
  ;[1 1 1] Tracking all the pellets in the level.
  (bind _outactors (Actor|GetAllActorsOfClass "/Game/Blueprints/Collectibles/BP_Collectible.BP_Collectible_C"))
  (Variables|Default|SetPellets _outactors))

(event EventTick
  (params (DeltaSeconds :type Float%20%28single-precision%29))
  ;[1 1 1] Handling when there are no more pellets to collect.
  (if (== (Utilities|Array|Length (Variables|Default|GetPellets)) 0)
    (CallFunction|RegenerateLevel)))

(fn ConstructionScript)

(fn AddPoints
  (params (pointsToAdd :type Integer))
  (Variables|Default|SettotalPoints (+ pointsToAdd (Variables|Default|GettotalPoints))))

(fn OnDeath
  (params (playerPawn :type Pawn%20Object%20Reference)))