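; Player controller that lets input from one controller steer two Pac-Man pawns for local play.
; On BeginPlay it caches all BP_PacMan actors and adds the IM_PlayerWASD Enhanced Input mapping context.
; MoveWASD and MoveArrows set MoveDirection on the first and second cached Pac-Man respectively, relying on GetAllActorsOfClass order.
; Directions are restricted to one axis, with X taking priority over Y and zero input ignored.
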(event Input|EnhancedActionEvents|EnhancedInputActionMoveArrows
  (params (ActionValue :type Vector%202D%20Structure) (ElapsedSeconds :type Float%20%28double-precision%29) (TriggeredSeconds :type Float%20%28double-precision%29) (InputAction :type Input%20Action%20Object%20Reference :default "/Game/Blueprints/Input/MoveArrows.MoveArrows"))
  (bind (_x _y) (Math|Vector2D|BreakVector2D ActionValue))
  (bind _pacmans (Variables|Default|GetPacMans))
  (bind _output (Utilities|Array|Get(acopy) _pacmans 1))
  ;[1 1 1] Setting move direction when an input is triggered.
  (:Triggered
    (if (!= _x 0.0)
      (Variables|/Game/Blueprints/CharacterPawns/BP_PacMan.BP_PacMan_C|SetmoveDirection _output (Math|Vector|MakeVector _x 0.0 0.0))
      (elif (!= _y 0.0)
        (Variables|/Game/Blueprints/CharacterPawns/BP_PacMan.BP_PacMan_C|SetmoveDirection _output (Math|Vector|MakeVector 0.0 _y 0.0))))))

(event Input|EnhancedActionEvents|EnhancedInputActionMoveWASD
  (params (ActionValue :type Vector%202D%20Structure) (ElapsedSeconds :type Float%20%28double-precision%29) (TriggeredSeconds :type Float%20%28double-precision%29) (InputAction :type Input%20Action%20Object%20Reference :default "/Game/Blueprints/Input/MoveWASD.MoveWASD"))
  (bind (_x _y) (Math|Vector2D|BreakVector2D ActionValue))
  (bind _pacmans (Variables|Default|GetPacMans))
  (bind _output (Utilities|Array|Get(acopy) _pacmans))
  ;[1 1 1] Setting move direction when an input is triggered.
  (:Triggered
    (if (!= _x 0.0)
      (Variables|/Game/Blueprints/CharacterPawns/BP_PacMan.BP_PacMan_C|SetmoveDirection _output (Math|Vector|MakeVector _x 0.0 0.0))
      (elif (!= _y 0.0)
        (Variables|/Game/Blueprints/CharacterPawns/BP_PacMan.BP_PacMan_C|SetmoveDirection _output (Math|Vector|MakeVector 0.0 _y 0.0))))))

(event EventBeginPlay
  (bind _outactors (Actor|GetAllActorsOfClass "/Game/Blueprints/CharacterPawns/BP_PacMan.BP_PacMan_C"))
  (Variables|Default|SetPacMans _outactors)
  (Input|AddMappingContext (PlayerController|LocalPlayerSubsystems|GetEnhancedInputLocalPlayerSubsystem self) "/Game/Blueprints/Input/IM_PlayerWASD.IM_PlayerWASD" 0 "(bIgnoreAllPressedKeysUntilRelease=True,bForceImmediately=False)"))

(fn ConstructionScript)