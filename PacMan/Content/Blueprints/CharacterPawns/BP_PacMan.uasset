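; Player Pac-Man pawn that moves on one axis at a time, collects pellets, and eats or dies to ghosts.
; Enhanced Input sets a direction that Tick applies without sweep, pausing while ShouldDelay is set.
; Sphere overlaps award points, trigger timed ghost scattering from power pellets, and score scattering ghosts with doubling values.
; Losing a life updates the UI and game mode, then respawns everyone or opens the main menu.
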(event OnComponentBeginOverlap(Sphere)
  (params (OverlappedComponent :type Primitive%20Component%20Object%20Reference) (OtherActor :type Actor%20Object%20Reference) (OtherComp :type Primitive%20Component%20Object%20Reference) (OtherBodyIndex :type Integer) (bFromSweep :type Boolean) (SweepResult :type Hit%20Result%20Structure%20%28by%20ref%29))
  (Utilities|FlowControl|Sequence
    (:then_0
      ;[1 1 1] Checking for collisions with collectibles.
      (if (Utilities|ClassIsChildOf (Utilities|GetClass OtherActor) "/Game/Blueprints/Collectibles/BP_Collectible.BP_Collectible_C")
        (Utilities|FlowControl|Sequence
          (:then_0
            (bind _aspac_man_game_mode (Utilities|Casting|CastToPacManGameMode (Game|GetGameMode)))
            (bind _asbp_collectible (Utilities|Casting|CastToBP_Collectible OtherActor))
            (Variables|Default|Setpoints (+ (Variables|Default|Getpoints) (Variables|/Game/Blueprints/Collectibles/BP_Collectible.BP_Collectible_C|Getpoints _asbp_collectible)))
            (Actor|DestroyActor _asbp_collectible)
            (Utilities|Array|RemoveItem (Variables|/Game/Blueprints/GameModes/PacManGameMode.PacManGameMode_C|GetPellets _aspac_man_game_mode) _asbp_collectible)
            ;[1 1 1] Setting chomp sound to delay and not overlap.
            (if (Variables|Default|GetshouldChomp)
              (Utilities|FlowControl|DoOnce false :!label _label
                (:Completed
                  (Audio|PlaySound2D "/Game/Sounds/pacman_chomp.pacman_chomp" 1.0 1.0 0.0 0 0 false)
                  (Variables|Default|SetshouldChomp false)
                  (Utilities|FlowControl|Delay 0.25)
                  (Variables|Default|SetshouldChomp true)
                  (goto _label Reset)))))
          (:then_1
            ;;[0 0 0] If a power pellet, power up pac man.
            (if (== (Utilities|GetClass OtherActor) "/Game/Blueprints/Collectibles/BP_PowerPellet.BP_PowerPellet_C")
              (Utilities|PowerUpReset))))))
    (:then_1
      ;[1 0.276 0.276] Checking for collisions with ghosts.
      (if (Utilities|ClassIsChildOf (Utilities|GetClass OtherActor) "/Game/Blueprints/Ghost/Pawns/BP_Ghost.BP_Ghost_C")
        (bind _asbp_ghost (Utilities|Casting|CastToBP_Ghost OtherActor))
        (if (Variables|/Game/Blueprints/Ghost/Controllers/BP_GhostController.BP_GhostController_C|GetIsScattering (Variables|/Game/Blueprints/Ghost/Pawns/BP_Ghost.BP_Ghost_C|GetGhostController _asbp_ghost))
          (Transformation|SetActorLocation _asbp_ghost (Variables|/Game/Blueprints/Ghost/Pawns/BP_Ghost.BP_Ghost_C|GetStartLocation _asbp_ghost) false false)
          (Variables|/Game/Blueprints/Ghost/Controllers/BP_GhostController.BP_GhostController_C|SetIsScattering (Variables|/Game/Blueprints/Ghost/Pawns/BP_Ghost.BP_Ghost_C|GetGhostController _asbp_ghost) false)
          (CallFunction|AddGhostPoints)
          (else
            (Utilities|FlowControl|DoOnce false :!label _label_2
              (:Completed
                (Utilities|LifeLost
                  (:outputExec
                    (goto _label_2 Reset)))))))))))

(event Input|EnhancedActionEvents|EnhancedInputActionMove
  (params (ActionValue :type Vector%202D%20Structure) (ElapsedSeconds :type Float%20%28double-precision%29) (TriggeredSeconds :type Float%20%28double-precision%29) (InputAction :type Input%20Action%20Object%20Reference :default "/Game/Blueprints/Input/Move.Move"))
  (bind (_x _y) (Math|Vector2D|BreakVector2D ActionValue))
  ;[1 1 1] Setting move direction when an input is triggered.
  (:Triggered
    (if (!= _x 0.0)
      (Variables|Default|SetmoveDirection (Math|Vector|MakeVector _x 0.0 0.0))
      (elif (!= _y 0.0)
        (Variables|Default|SetmoveDirection (Math|Vector|MakeVector 0.0 _y 0.0))))))

(event EventBeginPlay
  (Utilities|FlowControl|Delay 5.2)
  ;[1 1 1] Hooking up input action context to the player controller.
  (bind _asplayer_controller (Utilities|Casting|CastToPlayerController (Pawn|GetController)))
  (Input|AddMappingContext (PlayerController|LocalPlayerSubsystems|GetEnhancedInputLocalPlayerSubsystem _asplayer_controller) "/Game/Blueprints/Input/Player.Player" 0 "(bIgnoreAllPressedKeysUntilRelease=True,bForceImmediately=False)")
  ;[1 1 1] Adding the UI widget to PacMan
  (bind _returnvalue (UserInterface|CreateWidget "/Game/Blueprints/UI/BP_GameUI.BP_GameUI_C" (Game|GetPlayerController 0)))
  (bind _output_get (Variables|Default|SetuiWidget _returnvalue))
  (UserInterface|Viewport|AddtoViewport _output_get 0))

(event EventTick
  (params (DeltaSeconds :type Float%20%28single-precision%29))
  ;[1 1 1] Handling movement.
  (if (Variables|Default|GetshouldDelay)
    (Utilities|FlowControl|DoOnce false :!label _label
      (:Completed
        (Variables|Default|SetmoveDirection "0, 0, 0")
        (bind _aspac_man_game_mode (Utilities|Casting|CastToPacManGameMode (Game|GetGameMode)))
        (Utilities|FlowControl|Delay (Variables|/Game/Blueprints/GameModes/PacManGameMode.PacManGameMode_C|GetRespawnDelay _aspac_man_game_mode))
        (Variables|Default|SetshouldDelay false)
        (goto _label Reset)))
    (else
      (CallFunction|Move (Variables|Default|GetmoveDirection) DeltaSeconds))))

(fn ConstructionScript)

(fn Move
  (params (moveDirection :type Vector) (deltaTime :type Float%20%28double-precision%29))
  (bind _sphere (Variables|Default|GetSphere))
  (bind _movespeed (Variables|Default|GetmoveSpeed))
  (bind _returnvalue (* deltaTime _movespeed))
  ;[1 1 1] Setting location based on move direction.
  (Transformation|SetWorldLocation _sphere (+ (Transformation|GetWorldLocation _sphere) (* moveDirection (Math|Vector|MakeVector _returnvalue _returnvalue 1.0))) false false))

(fn ResettoSpawn
  ;[1 1 1] Setting move direction to 0 and resetting to spawn.
  (Variables|Default|SetmoveDirection "0, 0, 0")
  (Transformation|SetWorldLocation (Variables|Default|GetSphere) (Variables|Default|GetspawnLocation) false false))

(fn AddGhostPoints
  (if (== (Variables|Default|GetcurrentGhostPoints) 0)
    ;[1 1 1] If a ghost hasn't been eaten yet, set the points to 200.
    (bind _output_get (Variables|Default|SetcurrentGhostPoints 200))
    (Variables|Default|Setpoints (+ _output_get (Variables|Default|Getpoints)))
    (else
      ;[1 1 1] If a ghost has been eaten already, double the point value collected
      (bind _output_get_2 (Variables|Default|SetcurrentGhostPoints (* (Variables|Default|GetcurrentGhostPoints) 2)))
      (Variables|Default|Setpoints (+ (Variables|Default|Getpoints) _output_get_2)))))