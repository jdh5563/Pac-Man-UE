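; BP_PacMan is the player-controlled Pac-Man pawn, driven by Enhanced Input.
; Input stores a single-axis direction, and Tick keeps shifting the Sphere along it by MoveSpeed, without sweep or delta-time scaling.
; Sphere overlaps award collectible points through GM_BaseGameMode, destroy the collectible and remove it from Pellets.
; Power pellets start a retriggerable delay that clears PoweredUp, while ghost hits only print a message.
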(event OnComponentBeginOverlap(Sphere)
  (params (OverlappedComponent :type Primitive%20Component%20Object%20Reference) (OtherActor :type Actor%20Object%20Reference) (OtherComp :type Primitive%20Component%20Object%20Reference) (OtherBodyIndex :type Integer) (bFromSweep :type Boolean) (SweepResult :type Hit%20Result%20Structure%20%28by%20ref%29))
  (Utilities|FlowControl|Sequence
    (:then_0
      ;[1 1 1] Checking for collisions with collectibles.
      (if (Utilities|ClassIsChildOf (Utilities|GetClass OtherActor) "/Game/Blueprints/Collectibles/BP_Collectible.BP_Collectible_C")
        (Utilities|FlowControl|Sequence
          (:then_0
            (bind _asgm_base_game_mode (Utilities|Casting|CastToGM_BaseGameMode (Game|GetGameMode)))
            (bind _asbp_collectible (Utilities|Casting|CastToBP_Collectible OtherActor))
            (Default|AddPoints _asgm_base_game_mode (Variables|/Game/Blueprints/Collectibles/BP_Collectible.BP_Collectible_C|Getpoints _asbp_collectible))
            (Actor|DestroyActor OtherActor)
            (Utilities|Array|RemoveItem (Variables|/Game/Blueprints/GM_BaseGameMode.GM_BaseGameMode_C|GetPellets _asgm_base_game_mode) _asbp_collectible))
          (:then_1
            ;;[0 0 0] If a power pellet, power up pac man.
            (if (== (Utilities|GetClass OtherActor) "/Game/Blueprints/Collectibles/BP_PowerPellet.BP_PowerPellet_C")
              (Utilities|PowerUpReset))))))
    (:then_1
      ;[1 0.276 0.276] Checking for collisions with ghosts.
      (if (Utilities|ClassIsChildOf (Utilities|GetClass OtherActor) "/Game/Blueprints/Ghost/BP_Ghost.BP_Ghost_C")
        (Development|PrintString "Hit by ghost.")))))

(event Input|EnhancedActionEvents|EnhancedInputActionMove
  (params (ActionValue :type Vector%202D%20Structure) (ElapsedSeconds :type Float%20%28double-precision%29) (TriggeredSeconds :type Float%20%28double-precision%29) (InputAction :type Input%20Action%20Object%20Reference :default "/Game/Blueprints/Input/Move.Move"))
  (bind (_x _y) (Math|Vector2D|BreakVector2D ActionValue))
  ;[1 1 1] Setting move direction when an input is triggered.
  (:Triggered
    (if (!= _x 0.0)
      (Variables|Default|SetmoveDirection (Math|Vector|MakeVector _x 0.0 0.0))
      (elif (!= _y 0.0)
        (Variables|Default|SetmoveDirection (Math|Vector|MakeVector 0.0 _y 0.0))))))

(event EventBeginPlay
  ;[1 1 1] Hooking up input action context to the player controller.
  (bind _asplayer_controller (Utilities|Casting|CastToPlayerController (Pawn|GetController)))
  (Input|AddMappingContext (PlayerController|LocalPlayerSubsystems|GetEnhancedInputLocalPlayerSubsystem _asplayer_controller) "/Game/Blueprints/Input/Player.Player" 0 "(bIgnoreAllPressedKeysUntilRelease=True,bForceImmediately=False)"))

(event EventTick
  (params (DeltaSeconds :type Float%20%28single-precision%29))
  (CallFunction|Move (Variables|Default|GetmoveDirection)))

(fn ConstructionScript)

(fn Move
  (params (moveDirection :type Vector))
  (bind _sphere (Variables|Default|GetSphere))
  (bind _movespeed (Variables|Default|GetmoveSpeed))
  (Transformation|SetWorldLocation _sphere (+ (* moveDirection (Math|Vector|MakeVector _movespeed _movespeed 1.0)) (Transformation|GetWorldLocation _sphere)) false false))